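; BP_Ceiling is an arrow projectile hazard that kills the player and sticks into what it hits.
; It plays an attached throw sound on spawn, and its DeathTrigger overlap calls the first-person character's DeathEvent once for Player-tagged actors.
; HitWall collisions with WorldStatic or Pawn objects halt physics and projectile movement.
; The first such hit also swaps the throw sound for an impact sound and destroys the arrow after a delay.
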(event `self.ReceiveBeginPlay`
  ;[0 0.2935 1] Play Sound on Begin Play
  (bind _returnvalue (`GameplayStatics.SpawnSoundAttached` "/Game/_USER/Sounds/ArrowSoundThrow.ArrowSoundThrow" (`self.Arrow`) "None" (0.0 0.0 0.0) (struct) "KeepRelativeOffset" true 1.0 1.0 0.0 null null))
  (set `self.SoundThrowRef` _returnvalue))

(event `self.DeathTrigger.OnComponentBeginOverlap`
  (params (OverlappedComponent :type "PrimitiveComponent Object Reference") (OtherActor :type "Actor Object Reference") (OtherComp :type "PrimitiveComponent Object Reference") (OtherBodyIndex :type Integer) (bFromSweep :type Boolean) (SweepResult :type "HitResult Structure (by ref)"))
  ;[0 0.3517 1] DeathTrigger collider calls Death Event
  (if (`self.ActorHasTag` OtherActor "Player")
    (`/Engine/EditorBlueprintResources/StandardMacros.DoOnce` false
      (:`Completed`
        (`/Game/FirstPersonBP/Blueprints/FirstPersonCharacter.DeathEvent` (cast `/Game/FirstPersonBP/Blueprints/FirstPersonCharacter` (`GameplayStatics.GetPlayerCharacter` 0) :!pure true))))))

(event `self.HitWall.OnComponentHit`
  (params (HitComponent :type "PrimitiveComponent Object Reference") (OtherActor :type "Actor Object Reference") (OtherComp :type "PrimitiveComponent Object Reference") (NormalImpulse :type "Vector Structure") (Hit :type "HitResult Structure (by ref)"))
  (bind _returnvalue (`PrimitiveComponent.GetCollisionObjectType` OtherComp))
  (bind _soundthrowref (`self.SoundThrowRef`))
  (bind _projectilemovement (`self.ProjectileMovement`))
  (bind _hitwall (`self.HitWall`))
  ;[0 0.2779 1] Stick Arrow to wall / Play sound on hit
  (if (or (`|EnumEquality` _returnvalue "ECC_WorldStatic") (`|EnumEquality` _returnvalue "ECC_Pawn"))
    (`PrimitiveComponent.SetSimulatePhysics` _hitwall false)
    (`PrimitiveComponent.SetEnableGravity` _hitwall false)
    (set `MovementComponent.Velocity` (0.0 0.0 0.0) _projectilemovement)
    (set `ProjectileMovementComponent.MaxSpeed` 0.0 (`self.ProjectileMovement`))
    (set `ProjectileMovementComponent.ProjectileGravityScale` 0.0 _projectilemovement)
    (`/Engine/EditorBlueprintResources/StandardMacros.DoOnce` false
      (:`Completed`
        (`GameplayStatics.SpawnSoundAtLocation` "/Game/_USER/Sounds/ArrowSoundHit.ArrowSoundHit" (`.ImpactPoint` (`GameplayStatics.BreakHitResult` Hit)) (struct) 1.0 1.0 0.0 null null)
        (if (`KismetSystemLibrary.IsValid` _soundthrowref)
          (`AudioComponent.Stop` _soundthrowref))
        (`KismetSystemLibrary.Delay` 5.0)
        (`self.K2_DestroyActor`)))))

(fn `UserConstructionScript`)