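; Ceiling trap zone that spawns BP_Spikes on a player standing in an active cell of its nine-cell grid.
; While the player overlaps Sphere9, a one-second looping timer shows one scene component per row of three and cycles each row's index.
; Box overlaps track occupied cells, spawning spikes below the scene component upon entering a visible cell or when the timer activates an occupied one.
; An older sequential-drop chain is disconnected.
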(event `self.Sphere9.OnComponentBeginOverlap`
  (params (OverlappedComponent :type "PrimitiveComponent Object Reference") (OtherActor :type "Actor Object Reference") (OtherComp :type "PrimitiveComponent Object Reference") (OtherBodyIndex :type Integer) (bFromSweep :type Boolean) (SweepResult :type "HitResult Structure (by ref)"))
  ;[1 1 1] Activate Timer On Overlap
  (if (`self.ActorHasTag` OtherActor "Player")
    (`self.RunningTrapEvent`)))

(event `RunningTrapEvent`
  ;[1 1 1] Timer
  (`KismetSystemLibrary.K2_SetTimer` null "TimerFunction" 1.0 true))

(event `self.Sphere9.OnComponentEndOverlap`
  (params (OverlappedComponent :type "PrimitiveComponent Object Reference") (OtherActor :type "Actor Object Reference") (OtherComp :type "PrimitiveComponent Object Reference") (OtherBodyIndex :type Integer))
  ;[1 1 1] Activate Timer On Overlap
  (if (`self.ActorHasTag` OtherActor "Player")
    (`KismetSystemLibrary.K2_ClearTimer` null "TimerFunction")))

(event `self.ReceiveBeginPlay`
  (bind _scenearray (`self.SceneArray`))
  (`KismetArrayLibrary.Array_Add` _scenearray (`self.Scene`))
  (`KismetArrayLibrary.Array_Add` _scenearray (`self.Scene1`))
  (`KismetArrayLibrary.Array_Add` _scenearray (`self.Scene2`))
  (`KismetArrayLibrary.Array_Add` _scenearray (`self.Scene3`))
  (`KismetArrayLibrary.Array_Add` _scenearray (`self.Scene4`))
  (`KismetArrayLibrary.Array_Add` _scenearray (`self.Scene5`))
  (`KismetArrayLibrary.Array_Add` _scenearray (`self.Scene6`))
  (`KismetArrayLibrary.Array_Add` _scenearray (`self.Scene7`))
  (`KismetArrayLibrary.Array_Add` _scenearray (`self.Scene8`))
  (set `self.ArrayQty` (- (`KismetArrayLibrary.Array_Length` (`self.SceneArray`)) 1)))

(event `self.ReceiveTick`
  (params (DeltaSeconds :type "Float (single-precision)")))

(event `self.Box.OnComponentBeginOverlap`
  (params (OverlappedComponent :type "PrimitiveComponent Object Reference") (OtherActor :type "Actor Object Reference") (OtherComp :type "PrimitiveComponent Object Reference") (OtherBodyIndex :type Integer) (bFromSweep :type Boolean) (SweepResult :type "HitResult Structure (by ref)"))
  (bind _scene (`self.Scene`))
  (if (`self.ActorHasTag` OtherActor "Player")
    (`KismetArrayLibrary.Array_Set` (`self.bInBox`) 0 true)
    (if (`SceneComponent.IsVisible` _scene)
      (`self.SpawnCeilings` (`SceneComponent.K2_GetComponentToWorld` _scene)))))

(event `self.Box1.OnComponentBeginOverlap`
  (params (OverlappedComponent :type "PrimitiveComponent Object Reference") (OtherActor :type "Actor Object Reference") (OtherComp :type "PrimitiveComponent Object Reference") (OtherBodyIndex :type Integer) (bFromSweep :type Boolean) (SweepResult :type "HitResult Structure (by ref)"))
  (bind _scene1 (`self.Scene1`))
  (if (`self.ActorHasTag` OtherActor "Player")
    (`KismetArrayLibrary.Array_Set` (`self.bInBox`) 1 true)
    (if (`SceneComponent.IsVisible` _scene1)
      (`self.SpawnCeilings` (`SceneComponent.K2_GetComponentToWorld` _scene1)))))

(event `self.Box2.OnComponentBeginOverlap`
  (params (OverlappedComponent :type "PrimitiveComponent Object Reference") (OtherActor :type "Actor Object Reference") (OtherComp :type "PrimitiveComponent Object Reference") (OtherBodyIndex :type Integer) (bFromSweep :type Boolean) (SweepResult :type "HitResult Structure (by ref)"))
  (bind _scene2 (`self.Scene2`))
  (if (`self.ActorHasTag` OtherActor "Player")
    (`KismetArrayLibrary.Array_Set` (`self.bInBox`) 2 true)
    (if (`SceneComponent.IsVisible` _scene2)
      (`self.SpawnCeilings` (`SceneComponent.K2_GetComponentToWorld` _scene2)))))

(event `self.Box3.OnComponentBeginOverlap`
  (params (OverlappedComponent :type "PrimitiveComponent Object Reference") (OtherActor :type "Actor Object Reference") (OtherComp :type "PrimitiveComponent Object Reference") (OtherBodyIndex :type Integer) (bFromSweep :type Boolean) (SweepResult :type "HitResult Structure (by ref)"))
  (bind _scene3 (`self.Scene3`))
  (if (`self.ActorHasTag` OtherActor "Player")
    (`KismetArrayLibrary.Array_Set` (`self.bInBox`) 3 true)
    (if (`SceneComponent.IsVisible` _scene3)
      (`self.SpawnCeilings` (`SceneComponent.K2_GetComponentToWorld` _scene3)))))

(event `self.Box4.OnComponentBeginOverlap`
  (params (OverlappedComponent :type "PrimitiveComponent Object Reference") (OtherActor :type "Actor Object Reference") (OtherComp :type "PrimitiveComponent Object Reference") (OtherBodyIndex :type Integer) (bFromSweep :type Boolean) (SweepResult :type "HitResult Structure (by ref)"))
  (bind _scene4 (`self.Scene4`))
  (if (`self.ActorHasTag` OtherActor "Player")
    (`KismetArrayLibrary.Array_Set` (`self.bInBox`) 4 true)
    (if (`SceneComponent.IsVisible` _scene4)
      (`self.SpawnCeilings` (`SceneComponent.K2_GetComponentToWorld` _scene4)))))

(event `self.Box5.OnComponentBeginOverlap`
  (params (OverlappedComponent :type "PrimitiveComponent Object Reference") (OtherActor :type "Actor Object Reference") (OtherComp :type "PrimitiveComponent Object Reference") (OtherBodyIndex :type Integer) (bFromSweep :type Boolean) (SweepResult :type "HitResult Structure (by ref)"))
  (bind _scene5 (`self.Scene5`))
  (if (`self.ActorHasTag` OtherActor "Player")
    (`KismetArrayLibrary.Array_Set` (`self.bInBox`) 5 true)
    (if (`SceneComponent.IsVisible` _scene5)
      (`self.SpawnCeilings` (`SceneComponent.K2_GetComponentToWorld` _scene5)))))

(event `self.Box6.OnComponentBeginOverlap`
  (params (OverlappedComponent :type "PrimitiveComponent Object Reference") (OtherActor :type "Actor Object Reference") (OtherComp :type "PrimitiveComponent Object Reference") (OtherBodyIndex :type Integer) (bFromSweep :type Boolean) (SweepResult :type "HitResult Structure (by ref)"))
  (bind _scene6 (`self.Scene6`))
  (if (`self.ActorHasTag` OtherActor "Player")
    (`KismetArrayLibrary.Array_Set` (`self.bInBox`) 6 true)
    (if (`SceneComponent.IsVisible` _scene6)
      (`self.SpawnCeilings` (`SceneComponent.K2_GetComponentToWorld` _scene6)))))

(event `self.Box7.OnComponentBeginOverlap`
  (params (OverlappedComponent :type "PrimitiveComponent Object Reference") (OtherActor :type "Actor Object Reference") (OtherComp :type "PrimitiveComponent Object Reference") (OtherBodyIndex :type Integer) (bFromSweep :type Boolean) (SweepResult :type "HitResult Structure (by ref)"))
  (bind _scene7 (`self.Scene7`))
  (if (`self.ActorHasTag` OtherActor "Player")
    (`KismetArrayLibrary.Array_Set` (`self.bInBox`) 7 true)
    (if (`SceneComponent.IsVisible` _scene7)
      (`self.SpawnCeilings` (`SceneComponent.K2_GetComponentToWorld` _scene7)))))

(event `self.Box8.OnComponentBeginOverlap`
  (params (OverlappedComponent :type "PrimitiveComponent Object Reference") (OtherActor :type "Actor Object Reference") (OtherComp :type "PrimitiveComponent Object Reference") (OtherBodyIndex :type Integer) (bFromSweep :type Boolean) (SweepResult :type "HitResult Structure (by ref)"))
  (bind _scene8 (`self.Scene8`))
  (if (`self.ActorHasTag` OtherActor "Player")
    (`KismetArrayLibrary.Array_Set` (`self.bInBox`) 8 true)
    (if (`SceneComponent.IsVisible` _scene8)
      (`self.SpawnCeilings` (`SceneComponent.K2_GetComponentToWorld` _scene8)))))

(event `self.Box.OnComponentEndOverlap`
  (params (OverlappedComponent :type "PrimitiveComponent Object Reference") (OtherActor :type "Actor Object Reference") (OtherComp :type "PrimitiveComponent Object Reference") (OtherBodyIndex :type Integer))
  (`KismetArrayLibrary.Array_Set` (`self.bInBox`)))

(event `self.Box1.OnComponentEndOverlap`
  (params (OverlappedComponent :type "PrimitiveComponent Object Reference") (OtherActor :type "Actor Object Reference") (OtherComp :type "PrimitiveComponent Object Reference") (OtherBodyIndex :type Integer))
  (`KismetArrayLibrary.Array_Set` (`self.bInBox`) 1))

(event `self.Box2.OnComponentEndOverlap`
  (params (OverlappedComponent :type "PrimitiveComponent Object Reference") (OtherActor :type "Actor Object Reference") (OtherComp :type "PrimitiveComponent Object Reference") (OtherBodyIndex :type Integer))
  (`KismetArrayLibrary.Array_Set` (`self.bInBox`) 2))

(event `self.Box3.OnComponentEndOverlap`
  (params (OverlappedComponent :type "PrimitiveComponent Object Reference") (OtherActor :type "Actor Object Reference") (OtherComp :type "PrimitiveComponent Object Reference") (OtherBodyIndex :type Integer))
  (`KismetArrayLibrary.Array_Set` (`self.bInBox`) 3))

(event `self.Box4.OnComponentEndOverlap`
  (params (OverlappedComponent :type "PrimitiveComponent Object Reference") (OtherActor :type "Actor Object Reference") (OtherComp :type "PrimitiveComponent Object Reference") (OtherBodyIndex :type Integer))
  (`KismetArrayLibrary.Array_Set` (`self.bInBox`) 4))

(event `self.Box5.OnComponentEndOverlap`
  (params (OverlappedComponent :type "PrimitiveComponent Object Reference") (OtherActor :type "Actor Object Reference") (OtherComp :type "PrimitiveComponent Object Reference") (OtherBodyIndex :type Integer))
  (`KismetArrayLibrary.Array_Set` (`self.bInBox`) 5))

(event `self.Box6.OnComponentEndOverlap`
  (params (OverlappedComponent :type "PrimitiveComponent Object Reference") (OtherActor :type "Actor Object Reference") (OtherComp :type "PrimitiveComponent Object Reference") (OtherBodyIndex :type Integer))
  (`KismetArrayLibrary.Array_Set` (`self.bInBox`) 6))

(event `self.Box7.OnComponentEndOverlap`
  (params (OverlappedComponent :type "PrimitiveComponent Object Reference") (OtherActor :type "Actor Object Reference") (OtherComp :type "PrimitiveComponent Object Reference") (OtherBodyIndex :type Integer))
  (`KismetArrayLibrary.Array_Set` (`self.bInBox`) 7))

(event `self.Box8.OnComponentEndOverlap`
  (params (OverlappedComponent :type "PrimitiveComponent Object Reference") (OtherActor :type "Actor Object Reference") (OtherComp :type "PrimitiveComponent Object Reference") (OtherBodyIndex :type Integer))
  (`KismetArrayLibrary.Array_Set` (`self.bInBox`) 8))

(fn `CheckInsideBox`
  (for (_array_element _array_index) (`self.bInBox`)
    (if _array_element
      (if (or (== _array_index (`self.FirstRowInt`)) (== _array_index (`self.SecondRowInt`)) (== _array_index (`self.ThirdRowInt`)))
        (`self.SpawnCeilings` (`SceneComponent.K2_GetComponentToWorld` (`|GetArrayItem` (`self.SceneArray`) _array_index)))))))

(fn `FirstRowSwitch`
  (bind _firstrowint (`self.FirstRowInt`))
  (if (== _firstrowint 2)
    (set `self.FirstRowInt` 0)
    (else
      (`/Engine/EditorBlueprintResources/StandardMacros.IncrementInt` _firstrowint))))

(fn `RunAllSwitches`
  (`self.FirstRowSwitch`)
  (`self.SecondRowSwitch`)
  (`self.ThirdRowSwitch`)
  (`KismetSystemLibrary.PrintString` (`KismetStringLibrary.Concat_StrStr` "First : " (`KismetStringLibrary.Conv_IntToString` (`self.FirstRowInt`))))
  (`KismetSystemLibrary.PrintString` (`KismetStringLibrary.Concat_StrStr` "Second : " (`KismetStringLibrary.Conv_IntToString` (`self.SecondRowInt`))))
  (`KismetSystemLibrary.PrintString` (`KismetStringLibrary.Concat_StrStr` "Third : " (`KismetStringLibrary.Conv_IntToString` (`self.ThirdRowInt`)))))

(fn `SecondRowSwitch`
  (bind _secondrowint (`self.SecondRowInt`))
  (if (== _secondrowint 5)
    (set `self.SecondRowInt` 3)
    (else
      (`/Engine/EditorBlueprintResources/StandardMacros.IncrementInt` _secondrowint))))

(fn `SpawnCeilings`
  (params (SpawnTransform :type "Transform Structure"))
  (`|SpawnActorFromClass` "/Game/_USER/Blueprints/BP_Spikes.BP_Spikes_C" (`KismetMathLibrary.MakeTransform` (`KismetMathLibrary.MakeVector` (.x (.location SpawnTransform)) (.y (.location SpawnTransform)) (- (.z (.location SpawnTransform)) 500.0)) (`KismetMathLibrary.MakeRotator` (.roll (.rotation SpawnTransform)) (.pitch (.rotation SpawnTransform)) (.yaw (.rotation SpawnTransform))) (2.7 2.7 1.0)) "Undefined" "OverrideRootScale" null null))

(fn `ThirdRowSwitch`
  (bind _thirdrowint (`self.ThirdRowInt`))
  (if (== _thirdrowint 8)
    (set `self.ThirdRowInt` 6)
    (else
      (`/Engine/EditorBlueprintResources/StandardMacros.IncrementInt` _thirdrowint))))

(fn `TimerFunction`
  (for (_array_element _array_index) (`self.SceneArray`)
    (if (or (== _array_index (`self.FirstRowInt`)) (== _array_index (`self.SecondRowInt`)) (== _array_index (`self.ThirdRowInt`)))
      (`SceneComponent.SetVisibility` _array_element true true)
      (else
        (`SceneComponent.SetVisibility` _array_element false true))))
  (`self.CheckInsideBox`)
  (`self.RunAllSwitches`))

(fn `UserConstructionScript`)