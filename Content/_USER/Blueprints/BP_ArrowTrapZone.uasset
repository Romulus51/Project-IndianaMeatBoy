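; Arrow trap zone that fires volleys of BP_Arrows while a player-tagged actor is inside its sphere trigger.
; BeginPlay caches the world transforms of thirteen scene components as fixed spawn points.
; Overlap begin and end toggle the firing flag, which Tick checks alongside an accumulated-time threshold intended to space volleys two seconds apart.
; Each volley resets the time and spawns an arrow at every cached transform.
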(event `self.ReceiveBeginPlay`
  (bind _setscenetransformsarray (`self.SetSceneTransformsArray`))
  (`KismetArrayLibrary.Array_Add` _setscenetransformsarray (`SceneComponent.K2_GetComponentToWorld` (`self.Scene`)))
  (`KismetArrayLibrary.Array_Add` _setscenetransformsarray (`SceneComponent.K2_GetComponentToWorld` (`self.Scene2`)))
  (`KismetArrayLibrary.Array_Add` _setscenetransformsarray (`SceneComponent.K2_GetComponentToWorld` (`self.Scene3`)))
  (`KismetArrayLibrary.Array_Add` _setscenetransformsarray (`SceneComponent.K2_GetComponentToWorld` (`self.Scene4`)))
  (`KismetArrayLibrary.Array_Add` _setscenetransformsarray (`SceneComponent.K2_GetComponentToWorld` (`self.Scene5`)))
  (`KismetArrayLibrary.Array_Add` _setscenetransformsarray (`SceneComponent.K2_GetComponentToWorld` (`self.Scene6`)))
  (`KismetArrayLibrary.Array_Add` _setscenetransformsarray (`SceneComponent.K2_GetComponentToWorld` (`self.Scene7`)))
  (`KismetArrayLibrary.Array_Add` _setscenetransformsarray (`SceneComponent.K2_GetComponentToWorld` (`self.Scene8`)))
  (`KismetArrayLibrary.Array_Add` _setscenetransformsarray (`SceneComponent.K2_GetComponentToWorld` (`self.Scene9`)))
  (`KismetArrayLibrary.Array_Add` _setscenetransformsarray (`SceneComponent.K2_GetComponentToWorld` (`self.Scene10`)))
  (`KismetArrayLibrary.Array_Add` _setscenetransformsarray (`SceneComponent.K2_GetComponentToWorld` (`self.Scene11`)))
  (`KismetArrayLibrary.Array_Add` _setscenetransformsarray (`SceneComponent.K2_GetComponentToWorld` (`self.Scene12`)))
  (`KismetArrayLibrary.Array_Add` _setscenetransformsarray (`SceneComponent.K2_GetComponentToWorld` (`self.Scene13`))))

(event `self.ReceiveTick`
  (params (DeltaSeconds :type "Float (single-precision)"))
  (bind _output_get (set `self.Delta Seconds` (+ DeltaSeconds (`self.Delta Seconds`))))
  (if (and (>= _output_get 2.0) (`self.PlaySpawnArrows`))
    (set `self.Delta Seconds` 0.0)
    (for _array_element (`self.SetSceneTransformsArray`)
      (`self.SpawnArrows` _array_element))))

(event `self.Sphere14.OnComponentBeginOverlap`
  (params (OverlappedComponent :type "PrimitiveComponent Object Reference") (OtherActor :type "Actor Object Reference") (OtherComp :type "PrimitiveComponent Object Reference") (OtherBodyIndex :type Integer) (bFromSweep :type Boolean) (SweepResult :type "HitResult Structure (by ref)"))
  (if (`self.ActorHasTag` OtherActor "Player")
    (set `self.PlaySpawnArrows` true)))

(event `self.Sphere14.OnComponentEndOverlap`
  (params (OverlappedComponent :type "PrimitiveComponent Object Reference") (OtherActor :type "Actor Object Reference") (OtherComp :type "PrimitiveComponent Object Reference") (OtherBodyIndex :type Integer))
  (if (`self.ActorHasTag` OtherActor "Player")
    (set `self.PlaySpawnArrows` false)))

(fn `SpawnArrows`
  (params (SpawnTransform :type "Transform Structure"))
  (`|SpawnActorFromClass` "/Game/_USER/Blueprints/BP_Arrows.BP_Arrows_C" SpawnTransform "Undefined" "OverrideRootScale" null null))

(fn `UserConstructionScript`)