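; A falling-ceiling destructible hazard that kills the player on contact with its DeathTrigger and destroys itself 15 seconds after BeginPlay.
; Destructible hits apply point damage to the hit actor, then share shake and sound logic with BoxShake hits.
; The camera shake respects the game instance toggle, the rockfall sound plays once, and impact sounds are throttled by a delayed boolean.
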(event `self.ReceiveBeginPlay`
  (`KismetSystemLibrary.Delay` 15.0)
  (`self.K2_DestroyActor`))

(event `self.Destructible.OnComponentHit`
  (params (HitComponent :type "PrimitiveComponent Object Reference") (OtherActor :type "Actor Object Reference") (OtherComp :type "PrimitiveComponent Object Reference") (NormalImpulse :type "Vector Structure") (Hit :type "HitResult Structure (by ref)"))
  (bind (_bblockinghit _binitialoverlap _time _distance _location _impactpoint _normal _impactnormal _physmat _hitactor) (`GameplayStatics.BreakHitResult` Hit))
  ;[0 0.4711 1] OnHit Destructs, shake and play sounds
  (`GameplayStatics.ApplyPointDamage` _hitactor 100.0 _impactpoint Hit null OtherActor "/Script/Engine.DamageType")
  (`self.CameraShakeFunction` :!label _label)
  (`|ExecutionSequence`
    (:`then_0`
      (`/Engine/EditorBlueprintResources/StandardMacros.DoOnce` false
        (:`Completed`
          (`GameplayStatics.PlaySoundAtLocation` "/Game/_USER/Sounds/RocksFallCue.RocksFallCue" _impactpoint (struct) 1.0 0.5 0.0 "/Game/_USER/Sounds/RocksAttenuation.RocksAttenuation" null null))))
    (:`then_1`
      (if (not (`self.bCanPlaySound`))
        (set `self.bCanPlaySound` true)
        (`GameplayStatics.PlaySoundAtLocation` "/Game/_USER/Sounds/RockImpactCue.RockImpactCue" _impactpoint (struct) 1.0 0.5 0.0 "/Game/_USER/Sounds/RocksAttenuation.RocksAttenuation" null null)
        (`KismetSystemLibrary.Delay` 1.0)
        (set `self.bCanPlaySound` false)))))

(event `self.BoxShake.OnComponentHit`
  (params (HitComponent :type "PrimitiveComponent Object Reference") (OtherActor :type "Actor Object Reference") (OtherComp :type "PrimitiveComponent Object Reference") (NormalImpulse :type "Vector Structure") (Hit :type "HitResult Structure (by ref)"))
  ;[0 0.4711 1] OnHit Destructs, shake and play sounds
  (goto _label))

(event `self.DeathTrigger.OnComponentBeginOverlap`
  (params (OverlappedComponent :type "PrimitiveComponent Object Reference") (OtherActor :type "Actor Object Reference") (OtherComp :type "PrimitiveComponent Object Reference") (OtherBodyIndex :type Integer) (bFromSweep :type Boolean) (SweepResult :type "HitResult Structure (by ref)"))
  ;[0 0.3517 1] DeathTrigger collider calls Death Event
  (if (`self.ActorHasTag` OtherActor "Player")
    (`/Engine/EditorBlueprintResources/StandardMacros.DoOnce` false
      (:`Completed`
        (`/Game/FirstPersonBP/Blueprints/FirstPersonCharacter.DeathEvent` (cast `/Game/FirstPersonBP/Blueprints/FirstPersonCharacter` (`GameplayStatics.GetPlayerCharacter` 0) :!pure true))))))

(fn `CameraShakeFunction`
  (bind _asind_meat_boy_instance (cast `/Game/_USER/IndMeatBoyInstance` (`GameplayStatics.GetGameInstance`)))
  (if (`/Game/_USER/IndMeatBoyInstance.bCameraShakeOn` _asind_meat_boy_instance)
    (`GameplayStatics.PlayWorldCameraShake` "/Game/_USER/CS_CeilingShake.CS_CeilingShake_C" (`self.K2_GetActorLocation`) 400.0 3000.0 1.0 true)))

(fn `UserConstructionScript`)