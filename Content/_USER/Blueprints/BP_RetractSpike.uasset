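; BP_RetractSpike is a spike trap that periodically pops out while the player is nearby and kills them on contact.
; A Sphere overlap toggles RetractSpike, which gates SetOffset, apparently driven by a looping timer started after a configurable delay.
; SetOffset plays an attenuated sound and a timeline that sweeps the mesh toward the Scene component's location.
; DeathTrigger calls the FirstPersonCharacter's DeathEvent through a DoOnce.
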(event `SetOffset`
  (if (`self.RetractSpike`)
    (`GameplayStatics.PlaySoundAtLocation` "/Game/_USER/Sound/SpikeTrap.SpikeTrap" (`self.K2_GetActorLocation`) (struct) 0.15 1.0 0.0 "/Game/_USER/Sounds/RocksAttenuation.RocksAttenuation" null null)
    (bind (_direction _move) (`Timeline|PopOutTimeline` :!via `PlayFromStart`)
      (:`Update`
        (`SceneComponent.K2_SetWorldLocation` (`self.SpikeMesh`) (`KismetMathLibrary.VLerp` (`self.WorldLocation`) (`self.TargetWorldLocation`) _move) true false)))))

(event `self.ReceiveBeginPlay`
  (set `self.WorldLocation` (`SceneComponent.K2_GetComponentLocation` (`self.SpikeMesh`)))
  (set `self.TargetWorldLocation` (`SceneComponent.K2_GetComponentLocation` (`self.Scene`)))
  (`KismetSystemLibrary.Delay` (`self.DelayB4Retract`))
  (`KismetSystemLibrary.K2_SetTimerDelegate` (`|CreateDelegate` :!event `SetOffset`) 4.0 true -1.0))

(event `self.DeathTrigger.OnComponentBeginOverlap`
  (params (OverlappedComponent :type "PrimitiveComponent Object Reference") (OtherActor :type "Actor Object Reference") (OtherComp :type "PrimitiveComponent Object Reference") (OtherBodyIndex :type Integer) (bFromSweep :type Boolean) (SweepResult :type "HitResult Structure (by ref)"))
  ;[0 0.3517 1] DeathTrigger collider calls Death Event
  (if (`self.ActorHasTag` OtherActor "Player")
    (`/Engine/EditorBlueprintResources/StandardMacros.DoOnce` false
      (:`Completed`
        (`/Game/FirstPersonBP/Blueprints/FirstPersonCharacter.DeathEvent` (cast `/Game/FirstPersonBP/Blueprints/FirstPersonCharacter` (`GameplayStatics.GetPlayerCharacter` 0) :!pure true))))))

(event `self.Sphere.OnComponentBeginOverlap`
  (params (OverlappedComponent :type "PrimitiveComponent Object Reference") (OtherActor :type "Actor Object Reference") (OtherComp :type "PrimitiveComponent Object Reference") (OtherBodyIndex :type Integer) (bFromSweep :type Boolean) (SweepResult :type "HitResult Structure (by ref)"))
  (if (`self.ActorHasTag` OtherActor "Player")
    (set `self.RetractSpike` true)))

(event `self.Sphere.OnComponentEndOverlap`
  (params (OverlappedComponent :type "PrimitiveComponent Object Reference") (OtherActor :type "Actor Object Reference") (OtherComp :type "PrimitiveComponent Object Reference") (OtherBodyIndex :type Integer))
  (if (`self.ActorHasTag` OtherActor "Player")
    (set `self.RetractSpike` false)))

(fn `UserConstructionScript`)