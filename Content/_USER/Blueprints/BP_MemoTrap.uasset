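; BP_MemoTrap is a destructible trap that collapses when hit or on a timed call, then plays a falling-rocks sound and destroys itself.
; DestroyOnTouch sets whether its Box ignores or blocks Pawns at start.
; CallTimelineToDestroy uses a Timeline as the countdown, restarting a running one only when the requested delay is shorter.
; Collapse turns on Sphere physics and disables Destructible collision; hits on the Destructible also apply point damage.
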(event `self.ReceiveBeginPlay`
  (bind _box (`self.Box`))
  (if (`self.bDestroyOnTouch`)
    (`PrimitiveComponent.SetCollisionResponseToChannel` _box "ECC_Pawn" "ECR_Ignore")
    (else
      (`PrimitiveComponent.SetCollisionResponseToChannel` _box "ECC_Pawn" "ECR_Block"))))

(event `CollapseMeshEvent`
  (bind _sphere (`self.Sphere`))
  (`PrimitiveComponent.SetEnableGravity` _sphere true)
  (`PrimitiveComponent.SetSimulatePhysics` _sphere true)
  (`KismetSystemLibrary.Delay` 0.3)
  (`PrimitiveComponent.SetCollisionEnabled` (`self.Destructible`) "NoCollision"))

(event `CallTimelineToDestroy`
  (params (DelayB4DestroyInSeconds :type "Float (double-precision)"))
  (bind _collapsetimeline (`self.CollapseTimeline`))
  (bind _collapsetimeline_2 (`self.CollapseTimeline`))
  (bind _returnvalue (/ 1.0 (`TimelineComponent.GetPlayRate` _collapsetimeline_2)))
  (if (`TimelineComponent.IsPlaying` _collapsetimeline_2)
    (if (> (- _returnvalue (* (`TimelineComponent.GetPlaybackPosition` _collapsetimeline_2) _returnvalue)) DelayB4DestroyInSeconds)
      (if (== DelayB4DestroyInSeconds 0.0)
        (`TimelineComponent.Stop` _collapsetimeline)
        (`self.CollapseMeshEvent` :!label _label)
        (`PrimitiveComponent.SetCollisionResponseToChannel` (`self.Box`) "ECC_Pawn" "ECR_Ignore")
        (`KismetSystemLibrary.Delay` 0.5)
        (`/Engine/EditorBlueprintResources/StandardMacros.DoOnce` false :!label _label_2
          (:`Completed`
            (`GameplayStatics.PlaySoundAtLocation` "/Game/_USER/Sounds/RocksFallCue.RocksFallCue" (`self.K2_GetActorLocation`) (struct) 1.0 0.5 0.0 "/Game/_USER/Sounds/RocksAttenuation.RocksAttenuation" null null)
            (`KismetSystemLibrary.Delay` 4.0)
            (`self.K2_DestroyActor`)))
        (else
          (`TimelineComponent.SetPlayRate` _collapsetimeline DelayB4DestroyInSeconds)
          (`Timeline|CollapseTimeline` :!via `PlayFromStart` :!label _label_3
            (:`Finished`
              (goto _label))))))
    (else
      (`TimelineComponent.SetPlayRate` _collapsetimeline_2 (/ 1.0 DelayB4DestroyInSeconds))
      (goto _label_3 :!via `PlayFromStart`))))

(event `self.Destructible.OnComponentHit`
  (params (HitComponent :type "PrimitiveComponent Object Reference") (OtherActor :type "Actor Object Reference") (OtherComp :type "PrimitiveComponent Object Reference") (NormalImpulse :type "Vector Structure") (Hit :type "HitResult Structure (by ref)"))
  (bind (_bblockinghit _binitialoverlap _time _distance _location _impactpoint _normal _impactnormal _physmat _hitactor) (`GameplayStatics.BreakHitResult` Hit))
  (`GameplayStatics.ApplyPointDamage` _hitactor 100.0 _impactpoint Hit null OtherActor "/Script/Engine.DamageType")
  (`self.CollapseMesh`)
  (goto _label_2))

(fn `CollapseMesh`
  (bind _sphere (`self.Sphere`))
  (`PrimitiveComponent.SetEnableGravity` _sphere true)
  (`PrimitiveComponent.SetSimulatePhysics` _sphere true)
  (`PrimitiveComponent.SetCollisionEnabled` (`self.Destructible`) "NoCollision"))

(fn `UserConstructionScript`)