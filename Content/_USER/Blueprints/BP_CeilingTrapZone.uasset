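; BP_CeilingTrapZone is a trap zone that spawns a series of destructible ceiling pieces once a Player-tagged actor enters its box.
; BeginPlay caches the world transforms of seven scene components as drop points.
; Tick accumulates time and, at each delay interval, increments an index and spawns a scaled BP_CeilingDestructible at that point, stopping once the index reaches the last one.
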(event `self.ReceiveBeginPlay`
  (bind _setscenetransformsarray (`self.SetSceneTransformsArray`))
  (`KismetArrayLibrary.Array_Add` _setscenetransformsarray (`SceneComponent.K2_GetComponentToWorld` (`self.Scene`)))
  (`KismetArrayLibrary.Array_Add` _setscenetransformsarray (`SceneComponent.K2_GetComponentToWorld` (`self.Scene2`)))
  (`KismetArrayLibrary.Array_Add` _setscenetransformsarray (`SceneComponent.K2_GetComponentToWorld` (`self.Scene3`)))
  (`KismetArrayLibrary.Array_Add` _setscenetransformsarray (`SceneComponent.K2_GetComponentToWorld` (`self.Scene4`)))
  (`KismetArrayLibrary.Array_Add` _setscenetransformsarray (`SceneComponent.K2_GetComponentToWorld` (`self.Scene5`)))
  (`KismetArrayLibrary.Array_Add` _setscenetransformsarray (`SceneComponent.K2_GetComponentToWorld` (`self.Scene6`)))
  (`KismetArrayLibrary.Array_Add` _setscenetransformsarray (`SceneComponent.K2_GetComponentToWorld` (`self.Scene7`)))
  (set `self.ArrayQty` (- (`KismetArrayLibrary.Array_Length` (`self.SetSceneTransformsArray`)) 1)))

(event `self.ReceiveTick`
  (params (DeltaSeconds :type "Float (single-precision)"))
  (bind _arrayplay (`self.ArrayPlay`))
  (bind _output_get (set `self.Delta Seconds` (+ DeltaSeconds (`self.Delta Seconds`))))
  (if (and (>= _output_get (`self.DelayDurationBetweenDrops`)) (`self.PlaySpawnCeilings`))
    (set `self.Delta Seconds` 0.0)
    (`/Engine/EditorBlueprintResources/StandardMacros.IncrementInt` _arrayplay
      (:`  `
        (`self.SpawnCeilings` (`|GetArrayItem` (`self.SetSceneTransformsArray`) _arrayplay))
        (if (not (< (`self.ArrayPlay`) (`self.ArrayQty`)))
          (set `self.PlaySpawnCeilings` false))))))

(event `self.Box.OnComponentBeginOverlap`
  (params (OverlappedComponent :type "PrimitiveComponent Object Reference") (OtherActor :type "Actor Object Reference") (OtherComp :type "PrimitiveComponent Object Reference") (OtherBodyIndex :type Integer) (bFromSweep :type Boolean) (SweepResult :type "HitResult Structure (by ref)"))
  (if (`self.ActorHasTag` OtherActor "Player")
    (set `self.PlaySpawnCeilings` true)))

(fn `SpawnCeilings`
  (params (SpawnTransform :type "Transform Structure"))
  (`|SpawnActorFromClass` "/Game/_USER/Blueprints/BP_CeilingDestructible.BP_CeilingDestructible_C" (`KismetMathLibrary.MakeTransform` SpawnTransform_Location SpawnTransform_Rotation (4.5 4.5 1.0)) "Undefined" "OverrideRootScale" null null))

(fn `UserConstructionScript`)