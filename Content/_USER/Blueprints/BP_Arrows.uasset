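; BP_Arrows is an arrow hazard that kills the player on contact.
; On BeginPlay it attaches a throw sound to the arrow and keeps a reference to it.
; The first DeathTrigger overlap with a Player-tagged actor calls DeathEvent on the FirstPersonCharacter, plays a hit sound at the impact point and stops the throw sound.
; The arrow then destroys itself after a short delay.
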(event `self.ReceiveBeginPlay`
  (bind _returnvalue (`GameplayStatics.SpawnSoundAttached` "/Game/_USER/Sounds/ArrowSoundThrow.ArrowSoundThrow" (`self.Arrow`) "None" (0.0 0.0 0.0) (struct) "KeepRelativeOffset" true 1.0 1.0 0.0 null null))
  (set `self.SoundThrowRef` _returnvalue))

(event `self.DeathTrigger.OnComponentBeginOverlap`
  (params (OverlappedComponent :type "PrimitiveComponent Object Reference") (OtherActor :type "Actor Object Reference") (OtherComp :type "PrimitiveComponent Object Reference") (OtherBodyIndex :type Integer) (bFromSweep :type Boolean) (SweepResult :type "HitResult Structure (by ref)"))
  (bind _soundthrowref (`self.SoundThrowRef`))
  ;[0 0.3517 1] DeathTrigger collider calls Death Event
  (if (`self.ActorHasTag` OtherActor "Player")
    (`/Engine/EditorBlueprintResources/StandardMacros.DoOnce` false
      (:`Completed`
        (`/Game/FirstPersonBP/Blueprints/FirstPersonCharacter.DeathEvent` (cast `/Game/FirstPersonBP/Blueprints/FirstPersonCharacter` (`GameplayStatics.GetPlayerCharacter` 0) :!pure true))
        (`GameplayStatics.SpawnSoundAtLocation` "/Game/_USER/Sounds/ArrowSoundHit.ArrowSoundHit" (`.ImpactPoint` (`GameplayStatics.BreakHitResult` SweepResult)) (struct) 1.0 1.0 0.0 null null)
        (if (`KismetSystemLibrary.IsValid` _soundthrowref)
          (`AudioComponent.Stop` _soundthrowref))
        (`KismetSystemLibrary.Delay` 2.0)
        (`self.K2_DestroyActor`)))))

(fn `UserConstructionScript`)